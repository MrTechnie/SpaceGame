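; Bot character Blueprint that lets the player pick up nearby items into an inventory.
; Pressing E loops through overlapping BP_Item actors and calls PickUpItemMessage on those implementing the BPI_PickUp interface.
; Each returned item goes to the BPCInventory component through AddItemToInventory.
; A disabled earlier version of the E handler remains in the graph, and the other events are empty.
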(event `Key|E`
  (params (Key :type "Key Structure"))
  (:`Pressed`
    (for _array_element (`self.GetOverlappingActors` "/Game/Inventory/BP_Item.BP_Item_C")
      (if (`KismetSystemLibrary.DoesImplementInterface` _array_element "/Game/Inventory/BPI_PickUp.BPI_PickUp_C")
        ;[1 1 1] returns our item
        (bind _item (message `/Game/Inventory/BPI_PickUp.PickUp Item` _array_element))
        (`/Game/Inventory/BPC_Inventory.Add Item To Inventory` (`self.BPC_Inventory`) _item)))))

(fn `UserConstructionScript`)